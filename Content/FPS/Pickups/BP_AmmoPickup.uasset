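; BP_AmmoPickup is a rotating, respawning pickup that gives a set amount of ammo for a weapon type.
; On sphere overlap it hides the mesh, plays a sound, swaps to an inactive collision profile and sends AddAmmoMessage to the overlapping actor without casting.
; A timer handles the respawn delay.
; Respawn restores the active state, mesh and collision, with a sound and Niagara effect.
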(event Custom|OnComponentBeginOverlap_Event
  (params (OverlappedComponent :type Primitive%20Component%20Object%20Reference) (OtherActor :type Actor%20Object%20Reference) (OtherComp :type Primitive%20Component%20Object%20Reference) (OtherBodyIndex :type Integer) (bFromSweep :type Boolean) (SweepResult :type Hit%20Result%20Structure%20%28by%20ref%29))
  (Variables|Default|SetOther%20Actor OtherActor)
  (if (Variables|Default|GetIsActive)
    (Utilities|FlowControl|Sequence
      (:then_0
        ;[0.15 0.15 0.15 0.5] Hide And Play Sound
        (Rendering|SetVisibility (Variables|Default|GetPickupMesh) false false)
        (Audio|PlaySoundatLocation (Variables|Default|GetPickup%20Sound) (Transformation|GetActorLocation) "0, 0, 0" 1.0 1.0 0.0 0 0 0 0))
      (:then_1
        ;[0.15 0.15 0.15 0.5] Disable Sphere Collision
        (Collision|SetCollisionProfileName (Variables|Default|GetSphere) (Variables|Default|GetInactive%20Collision%20Profile) true :!class /Script/Engine.PrimitiveComponent))
      (:then_2
        (Variables|Default|SetIsActive false))
      (:then_3
        ;[0.15 0.15 0.15 0.5] Add Ammo
        (Class|PlayerInterface|AddAmmo(Message) (Variables|Default|GetOther%20Actor) (Variables|Default|GetWeaponType) (Variables|Default|GetAmmo%20Amount)))
      (:then_4
        (bind _returnvalue (Utilities|Time|SetTimerbyEvent (EventDispatchers|CreateEvent :!event Custom|Respawn) (Variables|Default|GetRespawn%20Interval)))
        (Variables|Default|SetRespawn%20Timer _returnvalue)))))

(event Custom|Respawn
  (Utilities|FlowControl|Sequence
    (:then_0
      ;[0.15 0.15 0.15 0.5] Reactivate
      (Variables|Default|SetIsActive true))
    (:then_1
      ;[0.15 0.15 0.15 0.5] Show the mesh
      (Rendering|SetVisibility (Variables|Default|GetPickupMesh) true false))
    (:then_2
      ;[0.15 0.15 0.15 0.5] Reactivate Sphere Collision
      (Collision|SetCollisionProfileName (Variables|Default|GetSphere) (Variables|Default|GetActive%20Collision%20Profile) true :!class /Script/Engine.PrimitiveComponent))
    (:then_3
      ;[0.15 0.15 0.15 0.5] Play Sound
      (Audio|PlaySoundatLocation (Variables|Default|GetRespawn%20Sound) (Transformation|GetActorLocation) "0, 0, 0" 1.0 1.0 0.0 0 0 0 0)
      (Niagara|SpawnSystematLocation "/Game/Effects/Particles/Item/NS_GunPad_Pickup_2.NS_GunPad_Pickup_2" (+ (Transformation|GetActorLocation) "0.000000,0.000000,50.000000")))))

(event EventBeginPlay
  (Collision|AssignOnComponentBeginOverlap (Variables|Default|GetSphere) (delegate Custom|OnComponentBeginOverlap_Event)))

(event Collision|EventActorBeginOverlap
  (params (OtherActor :type Actor%20Object%20Reference)))

(event EventTick
  (params (DeltaSeconds :type Float%20%28single-precision%29))
  (if (Variables|Default|GetIsActive)
    (Transformation|AddWorldRotation (Variables|Default|GetPickupMesh) (Math|Rotator|MakeRotator 0.0 0.0 (* (Variables|Default|GetRotation%20Rate) (Utilities|Time|GetWorldDeltaSeconds))) false false)))

(fn ConstructionScript)